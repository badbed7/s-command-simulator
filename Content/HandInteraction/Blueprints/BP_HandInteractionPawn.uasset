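; VR hand-interaction pawn that lets each hand grab and release actors tagged "Cube" by grip, pinch or aim.
; Tick line-traces from each free hand's aim component, moving a hit point and recording aimed cubes.
; Grip and pinch inputs sphere-trace at the hand and send grab or release messages, with pinch falling back to the aimed cube.
; Ready and aim inputs only print debug strings.
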(event `self.ReceiveTick`
  (params (DeltaSeconds :type "Float (single-precision)"))
  (bind _hitpoint_r (`self.HitPoint_R`))
  (bind _hitpoint_l (`self.HitPoint_L`))
  (bind _aim_r (`self.Aim_R`))
  (bind _aim_l (`self.Aim_L`))
  (bind _returnvalue (`SceneComponent.K2_GetComponentLocation` _aim_l))
  (bind _returnvalue_2 (`SceneComponent.K2_GetComponentLocation` _aim_r))
  ;[0 0 0 1 30] Aim Interaction line trace
  (`|ExecutionSequence`
    (:`then_0`
      (if (not (`self.RightHandGrabing`))
        (bind _outactors (`GameplayStatics.GetAllActorsOfClass` "/Game/HandTracking/Blueprints/BP_RiggedHandRenderModel.BP_RiggedHandRenderModel_C"))
        (bind (_outhit _returnvalue_3) (`KismetSystemLibrary.LineTraceSingle` _returnvalue_2 (+ _returnvalue_2 (* (`SceneComponent.GetForwardVector` _aim_r) 1000.0)) "TraceTypeQuery1" false _outactors "None" true (struct :`R` 1.0 :`A` 1.0) (struct :`G` 1.0 :`A` 1.0) 1.0))
        (if _returnvalue_3
          (bind (_bblockinghit _binitialoverlap _time _distance _location _impactpoint _normal _impactnormal _physmat _hitactor _hitcomponent _hitbonename _bonename _hititem _elementindex _faceindex _tracestart _traceend) (`GameplayStatics.BreakHitResult` _outhit))
          (`SceneComponent.K2_SetWorldLocation` _hitpoint_r _location false false)
          (if (`self.ActorHasTag` _hitactor "Cube")
            (set `self.Right Hit Actor` _hitactor)
            (set `self.RightHandAimObject` true))
          (else
            (`SceneComponent.K2_SetWorldLocation` _hitpoint_r _traceend false false)
            (set `self.RightHandAimObject` false)
            (set `self.Right Hit Actor` null)))))
    (:`then_1`
      (if (not (`self.LeftHandGrabing`))
        (bind _outactors_2 (`GameplayStatics.GetAllActorsOfClass` "/Game/HandTracking/Blueprints/BP_RiggedHandRenderModel.BP_RiggedHandRenderModel_C"))
        (bind (_outhit_2 _returnvalue_4) (`KismetSystemLibrary.LineTraceSingle` _returnvalue (+ _returnvalue (* (`SceneComponent.GetForwardVector` _aim_l) 1000.0)) "TraceTypeQuery1" false _outactors_2 "None" true (struct :`R` 1.0 :`A` 1.0) (struct :`G` 1.0 :`A` 1.0) 1.0))
        (if _returnvalue_4
          (bind (_bblockinghit_2 _binitialoverlap_2 _time_2 _distance_2 _location_2 _impactpoint_2 _normal_2 _impactnormal_2 _physmat_2 _hitactor_2 _hitcomponent_2 _hitbonename_2 _bonename_2 _hititem_2 _elementindex_2 _faceindex_2 _tracestart_2 _traceend_2) (`GameplayStatics.BreakHitResult` _outhit_2))
          (`SceneComponent.K2_SetWorldLocation` _hitpoint_l _location_2 false false)
          (if (`self.ActorHasTag` _hitactor_2 "Cube")
            (set `self.Left Hit Actor` _hitactor_2)
            (set `self.LeftHandAimObject` true))
          (else
            (`SceneComponent.K2_SetWorldLocation` _hitpoint_l _traceend_2 false false)
            (set `self.LeftHandAimObject` false)
            (set `self.Left Hit Actor` null)))))))

(event `self.ReceiveBeginPlay`
  (`HeadMountedDisplayFunctionLibrary.SetTrackingOrigin` "Floor"))

(event `Key|Escape`
  (params (Key :type "Key Structure"))
  (:`Pressed`
    (`KismetSystemLibrary.QuitGame` null "Quit")))

(event `EnhancedInput|/Game/EnhancedInput/IA_Keys/IA_Keys_AimReady_R`
  (params (ActionValue :type Boolean) (ElapsedSeconds :type "Float (double-precision)") (TriggeredSeconds :type "Float (double-precision)") (InputAction :type "InputAction Object Reference" :default "/Game/EnhancedInput/IA_Keys/IA_Keys_AimReady_R.IA_Keys_AimReady_R"))
  ;[0 0 0 1 30] Interaction ready enhanced input
  (:`Started`
    (`KismetSystemLibrary.PrintString` "Right Aim Ready")))

(event `EnhancedInput|/Game/EnhancedInput/IA_Keys/IA_Keys_AimReady_L`
  (params (ActionValue :type Boolean) (ElapsedSeconds :type "Float (double-precision)") (TriggeredSeconds :type "Float (double-precision)") (InputAction :type "InputAction Object Reference" :default "/Game/EnhancedInput/IA_Keys/IA_Keys_AimReady_L.IA_Keys_AimReady_L"))
  ;[0 0 0 1 30] Interaction ready enhanced input
  (:`Started`
    (`KismetSystemLibrary.PrintString` "Left Aim Ready")))

(event `EnhancedInput|`
  (params (ActionValue :type Boolean) (ElapsedSeconds :type "Float (double-precision)") (TriggeredSeconds :type "Float (double-precision)"))
  (bind _returnvalue (`SceneComponent.K2_GetComponentLocation` (`self.MotionController_R_Grip`)))
  ;[0 0 0 1 30] Grip interaction enhanced input
  (:`Triggered`
    (`KismetSystemLibrary.Delay` 0.2)
    (if (`self.RightHandGrabing`)
      _
      (elif (>= ActionValue 0.5)
        (bind (_outhit _returnvalue_2) (`KismetSystemLibrary.SphereTraceSingle` _returnvalue _returnvalue 5.0 "TraceTypeQuery1"))
        (if _returnvalue_2
          (bind (_bblockinghit _binitialoverlap _time _distance _location _impactpoint _normal _impactnormal _physmat _hitactor) (`GameplayStatics.BreakHitResult` _outhit))
          (if (`self.ActorHasTag` _hitactor "Cube")
            (bind _output_get (set `self.Right Hit Actor` _hitactor))
            (`/Engine/EditorBlueprintResources/StandardMacros.IsValid` _output_get
              (:`Is Valid`
                (message `/Game/HandInteraction/Blueprints/IGrabbable.Grab` _output_get (`self.Grip_R`))
                (set `self.RightHandGrabing` true))
              (:`Is Not Valid`
                (set `self.Right Hit Actor` null :!label _label)
                (set `self.RightHandGrabing` false)))
            (else
              (message `/Game/HandInteraction/Blueprints/IGrabbable.Release` (`self.Right Hit Actor`) :!label _label_2)
              (goto _label))))
        (else
          (if (`self.RightHandGrabing`) :!label _label_3
            (goto _label_2))))))
  (:`Canceled`
    (goto _label_3))
  (:`Completed`
    (goto _label_3)))

(event `EnhancedInput|/Game/EnhancedInput/IA_Keys/IA_Keys_GripReady_R`
  (params (ActionValue :type Boolean) (ElapsedSeconds :type "Float (double-precision)") (TriggeredSeconds :type "Float (double-precision)") (InputAction :type "InputAction Object Reference" :default "/Game/EnhancedInput/IA_Keys/IA_Keys_GripReady_R.IA_Keys_GripReady_R"))
  ;[0 0 0 1 30] Interaction ready enhanced input
  (:`Started`
    (`KismetSystemLibrary.PrintString` "Right Grip Ready")))

(event `EnhancedInput|/Game/EnhancedInput/IA_Keys/IA_Keys_GripReady_L`
  (params (ActionValue :type Boolean) (ElapsedSeconds :type "Float (double-precision)") (TriggeredSeconds :type "Float (double-precision)") (InputAction :type "InputAction Object Reference" :default "/Game/EnhancedInput/IA_Keys/IA_Keys_GripReady_L.IA_Keys_GripReady_L"))
  ;[0 0 0 1 30] Interaction ready enhanced input
  (:`Started`
    (`KismetSystemLibrary.PrintString` "Left Grip Ready")))

(event `EnhancedInput|/Game/EnhancedInput/IA_Keys/IA_Keys_PinchReady_R`
  (params (ActionValue :type Boolean) (ElapsedSeconds :type "Float (double-precision)") (TriggeredSeconds :type "Float (double-precision)") (InputAction :type "InputAction Object Reference" :default "/Game/EnhancedInput/IA_Keys/IA_Keys_PinchReady_R.IA_Keys_PinchReady_R"))
  ;[0 0 0 1 30] Interaction ready enhanced input
  (:`Started`
    (`KismetSystemLibrary.PrintString` "Right Pinch Ready")))

(event `EnhancedInput|/Game/EnhancedInput/IA_Keys/IA_Keys_PinchReady_L`
  (params (ActionValue :type Boolean) (ElapsedSeconds :type "Float (double-precision)") (TriggeredSeconds :type "Float (double-precision)") (InputAction :type "InputAction Object Reference" :default "/Game/EnhancedInput/IA_Keys/IA_Keys_PinchReady_L.IA_Keys_PinchReady_L"))
  ;[0 0 0 1 30] Interaction ready enhanced input
  (:`Started`
    (`KismetSystemLibrary.PrintString` "Left Pinch Ready")))

(event `EnhancedInput|`
  (params (ActionValue :type Boolean) (ElapsedSeconds :type "Float (double-precision)") (TriggeredSeconds :type "Float (double-precision)"))
  (bind _returnvalue (`SceneComponent.K2_GetComponentLocation` (`self.MotionController_L_Grip`)))
  ;[0 0 0 1 30] Grip interaction enhanced input
  (:`Triggered`
    (`KismetSystemLibrary.Delay` 0.2)
    (if (`self.LeftHandGrabing`)
      _
      (elif (>= ActionValue 0.5)
        (bind (_outhit _returnvalue_2) (`KismetSystemLibrary.SphereTraceSingle` _returnvalue _returnvalue 5.0 "TraceTypeQuery1"))
        (if _returnvalue_2
          (bind (_bblockinghit _binitialoverlap _time _distance _location _impactpoint _normal _impactnormal _physmat _hitactor) (`GameplayStatics.BreakHitResult` _outhit))
          (if (`self.ActorHasTag` _hitactor "Cube")
            (bind _output_get (set `self.Left Hit Actor` _hitactor))
            (`/Engine/EditorBlueprintResources/StandardMacros.IsValid` _output_get
              (:`Is Valid`
                (message `/Game/HandInteraction/Blueprints/IGrabbable.Grab` _output_get (`self.Grip_L`))
                (set `self.LeftHandGrabing` true))
              (:`Is Not Valid`
                (set `self.Left Hit Actor` null :!label _label_4)
                (set `self.LeftHandGrabing` false)))
            (else
              (message `/Game/HandInteraction/Blueprints/IGrabbable.Release` (`self.Left Hit Actor`) :!label _label_5)
              (goto _label_4))))
        (else
          (if (`self.LeftHandGrabing`) :!label _label_6
            (goto _label_5))))))
  (:`Canceled`
    (goto _label_6))
  (:`Completed`
    (goto _label_6)))

(event `EnhancedInput|/Game/EnhancedInput/IA_Keys/IA_Keys_Aim_Interaction_R`
  (params (ActionValue :type "Float (double-precision)") (ElapsedSeconds :type "Float (double-precision)") (TriggeredSeconds :type "Float (double-precision)") (InputAction :type "InputAction Object Reference" :default "/Game/EnhancedInput/IA_Keys/IA_Keys_Aim_Interaction_R.IA_Keys_Aim_Interaction_R"))
  ;[0 0 0 1 30] Aim Interaction enhanced input
  (:`Started`
    (`KismetSystemLibrary.PrintString` (`KismetStringLibrary.Concat_StrStr` "Right Aim value : " (`KismetStringLibrary.Conv_DoubleToString` ActionValue)))))

(event `EnhancedInput|/Game/EnhancedInput/IA_Keys/IA_Keys_Aim_Interaction_L`
  (params (ActionValue :type "Float (double-precision)") (ElapsedSeconds :type "Float (double-precision)") (TriggeredSeconds :type "Float (double-precision)") (InputAction :type "InputAction Object Reference" :default "/Game/EnhancedInput/IA_Keys/IA_Keys_Aim_Interaction_L.IA_Keys_Aim_Interaction_L"))
  ;[0 0 0 1 30] Aim Interaction enhanced input
  (:`Started`
    (`KismetSystemLibrary.PrintString` (`KismetStringLibrary.Concat_StrStr` "Left Aim value : " (`KismetStringLibrary.Conv_DoubleToString` ActionValue)))))

(event `EnhancedInput|/Game/EnhancedInput/IA_Keys/IA_Keys_Pinch_Interaction_R`
  (params (ActionValue :type "Float (double-precision)") (ElapsedSeconds :type "Float (double-precision)") (TriggeredSeconds :type "Float (double-precision)") (InputAction :type "InputAction Object Reference" :default "/Game/EnhancedInput/IA_Keys/IA_Keys_Pinch_Interaction_R.IA_Keys_Pinch_Interaction_R"))
  (bind _right_hit_actor (`self.Right Hit Actor`))
  (bind _returnvalue (`SceneComponent.K2_GetComponentLocation` (`self.MotionController_R_Pinch`)))
  ;[0 0 0 1 30] Pinch & Aim interaction enhanced input
  (:`Triggered`
    (`KismetSystemLibrary.Delay` 0.2)
    (if (`self.RightHandGrabing`)
      _
      (elif (>= ActionValue 0.5)
        (bind (_outhit _returnvalue_2) (`KismetSystemLibrary.SphereTraceSingle` _returnvalue _returnvalue 5.0 "TraceTypeQuery1"))
        (if _returnvalue_2
          (bind (_bblockinghit _binitialoverlap _time _distance _location _impactpoint _normal _impactnormal _physmat _hitactor) (`GameplayStatics.BreakHitResult` _outhit))
          (if (`self.ActorHasTag` _hitactor "Cube")
            (bind _output_get (set `self.Right Hit Actor` _hitactor))
            (`/Engine/EditorBlueprintResources/StandardMacros.IsValid` _output_get
              (:`Is Valid`
                (message `/Game/HandInteraction/Blueprints/IGrabbable.Grab` _output_get (`self.Pinch_R`))
                (set `self.RightHandGrabing` true))
              (:`Is Not Valid`
                (set `self.Right Hit Actor` null :!label _label_7)
                (set `self.RightHandGrabing` false)))
            (else
              (if (`self.RightHandAimObject`) :!label _label_8
                (`/Engine/EditorBlueprintResources/StandardMacros.IsValid` _right_hit_actor
                  (:`Is Valid`
                    (message `/Game/HandInteraction/Blueprints/IGrabbable.Grab` _right_hit_actor (`self.HitPoint_R`))
                    (set `self.RightHandGrabing` true))
                  (:`Is Not Valid`
                    (goto _label_7))))))
          (else
            (goto _label_8)))
        (else
          (if (`self.RightHandGrabing`) :!label _label_9
            (message `/Game/HandInteraction/Blueprints/IGrabbable.Release` (`self.Right Hit Actor`))
            (goto _label_7))))))
  (:`Canceled`
    (goto _label_9))
  (:`Completed`
    (goto _label_9)))

(event `EnhancedInput|/Game/EnhancedInput/IA_Keys/IA_Keys_Pinch_Interaction_L`
  (params (ActionValue :type "Float (double-precision)") (ElapsedSeconds :type "Float (double-precision)") (TriggeredSeconds :type "Float (double-precision)") (InputAction :type "InputAction Object Reference" :default "/Game/EnhancedInput/IA_Keys/IA_Keys_Pinch_Interaction_L.IA_Keys_Pinch_Interaction_L"))
  (bind _left_hit_actor (`self.Left Hit Actor`))
  (bind _returnvalue (`SceneComponent.K2_GetComponentLocation` (`self.MotionController_L_Pinch`)))
  ;[0 0 0 1 30] Pinch & Aim interaction enhanced input
  (:`Triggered`
    (`KismetSystemLibrary.Delay` 0.2)
    (if (`self.LeftHandGrabing`)
      _
      (elif (>= ActionValue 0.5)
        (bind (_outhit _returnvalue_2) (`KismetSystemLibrary.SphereTraceSingle` _returnvalue _returnvalue 5.0 "TraceTypeQuery1"))
        (if _returnvalue_2
          (bind (_bblockinghit _binitialoverlap _time _distance _location _impactpoint _normal _impactnormal _physmat _hitactor) (`GameplayStatics.BreakHitResult` _outhit))
          (if (`self.ActorHasTag` _hitactor "Cube")
            (bind _output_get (set `self.Left Hit Actor` _hitactor))
            (`/Engine/EditorBlueprintResources/StandardMacros.IsValid` _output_get
              (:`Is Valid`
                (message `/Game/HandInteraction/Blueprints/IGrabbable.Grab` _output_get (`self.Pinch_L`))
                (set `self.LeftHandGrabing` true))
              (:`Is Not Valid`
                (set `self.Left Hit Actor` null :!label _label_10)
                (set `self.LeftHandGrabing` false)))
            (else
              (if (`self.LeftHandAimObject`) :!label _label_11
                (`/Engine/EditorBlueprintResources/StandardMacros.IsValid` _left_hit_actor
                  (:`Is Valid`
                    (message `/Game/HandInteraction/Blueprints/IGrabbable.Grab` _left_hit_actor (`self.HitPoint_L`))
                    (set `self.LeftHandGrabing` true))
                  (:`Is Not Valid`
                    (goto _label_10))))))
          (else
            (goto _label_11)))
        (else
          (if (`self.LeftHandGrabing`) :!label _label_12
            (message `/Game/HandInteraction/Blueprints/IGrabbable.Release` (`self.Left Hit Actor`))
            (goto _label_10))))))
  (:`Canceled`
    (goto _label_12))
  (:`Completed`
    (goto _label_12)))

(fn `UserConstructionScript`)