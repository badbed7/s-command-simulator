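; Hand-tracking render model that adds collision-driven fingertip IK to a rigged hand.
; Each joint update sweeps five sphere colliders to their finger bones, retrying from along the hit normal when blocked and snapping to the bone if still overlapping.
; Collider-to-bone offsets, with length-clamped alphas, become IK goals passed alongside joint rotations to AnimBP update events.
; Those events and AnimBP setup are empty hooks here.
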(event `self.ReceiveBeginPlay`
  (`parent.ReceiveBeginPlay`)
  (set `self.FingerColliderToBone` (`|MakeMap` (`self.Sphere_WaveBone_5_Phy`) "WaveBone_5" (`self.Sphere_WaveBone_10_Phy`) "WaveBone_10" (`self.Sphere_WaveBone_15_Phy`) "WaveBone_15" (`self.Sphere_WaveBone_20_Phy`) "WaveBone_20" (`self.Sphere_WaveBone_25_Phy`) "WaveBone_25" :!type "SceneComponent Object Reference" :!valuetype "Name"))
  (`self.SetupAnimBPInst`))

(event `SetupAnimBPInst`)

(event `UpdateAnimBP_IKRigPos`
  (bind _fingercollidertobone (`self.FingerColliderToBone`))
  (bind _keys (`BlueprintMapLibrary.Map_Keys` _fingercollidertobone))
  (bind _values (`BlueprintMapLibrary.Map_Values` _fingercollidertobone))
  (for (_array_element _array_index) _keys
    (bind _output (`|GetArrayItem` _values _array_index))
    (bind _returnvalue (- (`SceneComponent.K2_GetComponentLocation` _array_element) (`SceneComponent.GetSocketLocation` (`self.PoseableMesh_Hand`) _output)))
    (`self.UpdateAnimBP_GoalPosition` _output _returnvalue (`KismetMathLibrary.FClamp` (`KismetMathLibrary.VSize` _returnvalue)))))

(event `UpdateAnimBP_JointRotation`
  (params (EHandKeypoint :type "EHandKeypoint Enum" :default "Palm") (InRotation :type "Rotator Structure")))

(event `UpdateAnimBP_GoalPosition`
  (params (BoneName :type Name) (`Goal Position` :type "Vector Structure") (`Goal Position Alpha` :type "Float (double-precision)")))

(fn `UpdateHandJointsTransform`
  (bind _fingercollidertobone (`self.FingerColliderToBone`))
  (`parent.UpdateHandJointsTransform`)
  (bind _keys (`BlueprintMapLibrary.Map_Keys` _fingercollidertobone))
  (bind _values (`BlueprintMapLibrary.Map_Values` _fingercollidertobone))
  (for (_array_element _array_index) _keys
    (bind _returnvalue (`SceneComponent.GetSocketLocation` (`self.PoseableMesh_Hand`) (`|GetArrayItem` _values _array_index)))
    (bind _sweephitresult (`SceneComponent.K2_SetWorldLocation` _array_element _returnvalue true false))
    (bind (_bblockinghit _binitialoverlap _time _distance _location _impactpoint _normal _impactnormal) (`GameplayStatics.BreakHitResult` _sweephitresult))
    (if _bblockinghit
      (`SceneComponent.K2_SetWorldLocation` _array_element (+ _returnvalue (* _impactnormal (`self.OverlapDistanceToDisableFingerIK`))) false true)
      (bind _sweephitresult_2 (`SceneComponent.K2_SetWorldLocation` _array_element _returnvalue true false))
      (if (`.bInitialOverlap` (`GameplayStatics.BreakHitResult` _sweephitresult_2))
        (`SceneComponent.K2_SetWorldLocation` _array_element _returnvalue false true))))
  (`self.UpdateAnimBP_IKRigPos`))

(fn `UpdateHandJointTransformToMesh`
  (params (EHandKeypoint :type "EHandKeypoint Enum" :default "Palm") (BoneName :type Name) (JointLocation :type "Vector Structure") (JointRotation :type "Rotator Structure"))
  (`parent.UpdateHandJointTransformToMesh` EHandKeypoint BoneName JointLocation JointRotation)
  (`self.UpdateAnimBP_JointRotation` EHandKeypoint JointRotation))

(fn `UserConstructionScript`
  (`parent.UserConstructionScript`))